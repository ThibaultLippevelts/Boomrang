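; BP_Movable_Box is a box that teleports to the player's position when a boomerang hits it.
; It caches the BP_ThirdPersonCharacter at BeginPlay, then on a Cube hit by BP_Boomerang moves its Box and Cube components to that character's location and calls the character's TP function.
; A CanTp flag with a short delay acts as a cooldown between teleports.
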(event OnComponentHit(Cube)
  (params (HitComponent :type Primitive%20Component%20Object%20Reference) (OtherActor :type Actor%20Object%20Reference) (OtherComp :type Primitive%20Component%20Object%20Reference) (NormalImpulse :type Vector :default "0, 0, 0") (Hit :type Hit%20Result%20Structure%20%28by%20ref%29))
  (bind _player_ref (Variables|Default|GetPlayer%20ref))
  (Utilities|Casting|CastToBP_Boomerang OtherActor)
  (if (Variables|Default|GetCan%20tp%20?)
    (Transformation|SetWorldLocation (Variables|Default|GetBox) (Transformation|GetActorLocation _player_ref) false true)
    (Default|TP _player_ref)
    (Variables|Default|SetCan%20tp%20? false)
    (Utilities|FlowControl|Delay 1.0)
    (Variables|Default|SetCan%20tp%20? true)))

(event EventBeginPlay
  (|CallParentFunction)
  (bind _returnvalue (Actor|GetActorOfClass "/Game/ThirdPerson/Blueprints/BP_ThirdPersonCharacter.BP_ThirdPersonCharacter_C"))
  (Variables|Default|SetPlayer%20ref _returnvalue)
  (Variables|Default|SetCan%20tp%20? true))

(fn ConstructionScript
  (|CallParentFunction))