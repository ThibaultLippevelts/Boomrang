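; BP_Boomerang is a thrown projectile that homes back to the third-person player character.
; On BeginPlay it takes its initial speed from BP_GI, then after a delay sets homing on the player's capsule.
; The first player overlap arms CanBeDestroyed; the next destroys the boomerang and re-enables CanShoot.
; The cached BP_Movable_Parents reference feeds only unconnected debug logic; other overlaps just print.
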(event OnComponentBeginOverlap(Sphere1)
  (params (OverlappedComponent :type Primitive%20Component%20Object%20Reference) (OtherActor :type Actor%20Object%20Reference) (OtherComp :type Primitive%20Component%20Object%20Reference) (OtherBodyIndex :type Integer) (bFromSweep :type Boolean) (SweepResult :type Hit%20Result%20Structure%20%28by%20ref%29))
  (if (== OtherActor (Variables|Default|GetAs%20BP%20Third%20Person%20Character))
    (Development|PrintString (Utilities|String|ToString(Boolean) (Variables|Default|Getcan%20be%20destroyed)))
    (if (Variables|Default|Getcan%20be%20destroyed)
      (Variables|Default|Setcan%20be%20destroyed false)
      (Variables|/Script/Engine.ProjectileMovementComponent|SetbIsHomingProjectile (Variables|Default|GetProjectileMovement) false)
      (Variables|/Game/ThirdPerson/Blueprints/BP_ThirdPersonCharacter.BP_ThirdPersonCharacter_C|Setcan%20shoot (Variables|Default|GetAs%20BP%20Third%20Person%20Character) true)
      (Actor|DestroyActor)
      (else
        (Variables|Default|Setcan%20be%20destroyed true)))
    (else
      (Development|PrintString "AAAAAAAAAAAAAAAAAAAAAA"))))

(event Custom|return
  (bind _projectilemovement (Variables|Default|GetProjectileMovement))
  (Variables|/Script/Engine.ProjectileMovementComponent|SetHomingTargetComponent _projectilemovement (Variables|/Script/Engine.Character|GetCapsuleComponent (Variables|Default|GetAs%20BP%20Third%20Person%20Character)))
  (Variables|/Script/Engine.ProjectileMovementComponent|SetbIsHomingProjectile _projectilemovement true))

(event Custom|update%20variable
  (Development|PrintString "Update")
  (bind _asbp_gi (Utilities|Casting|CastToBP_GI (Game|GetGameInstance)))
  (Variables|/Script/Engine.ProjectileMovementComponent|SetInitialSpeed (Variables|Default|GetProjectileMovement) (Variables|/Game/BP/BP_GI.BP_GI_C|GetSpeed _asbp_gi)))

(event EventBeginPlay
  (CallFunction|UpdateVariable)
  (bind _returnvalue (Actor|GetActorOfClass "/Game/BP/BP_Movable_Object/BP_Movable_Parents.BP_Movable_Parents_C"))
  (Variables|Default|SetMovable%20object _returnvalue)
  (Variables|Default|Setis%20destroy false)
  (Variables|Default|Setcan%20be%20destroyed false)
  (bind _asbp_third_person_character (Utilities|Casting|CastToBP_ThirdPersonCharacter (Game|GetPlayerCharacter 0)))
  (Variables|Default|SetAs%20BP%20Third%20Person%20Character _asbp_third_person_character)
  (Utilities|FlowControl|Delay (Variables|Default|GetDelay))
  (CallFunction|Return))

(fn ConstructionScript)