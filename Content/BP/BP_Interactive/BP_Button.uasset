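; BP_Button is an interactive switch that the boomerang triggers by touching it.
; On actor overlap it compares the other actor to the BP_Boomerang found by GetActorOfClass, so it responds only to that one instance.
; A match calls SwitchActivated on both the referenced DoorToOpen and BridgeToSpawn, then destroys the button's Box component.
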(event Collision|EventActorBeginOverlap
  (params (OtherActor :type Actor%20Object%20Reference))
  (bind _returnvalue (Actor|GetActorOfClass "/Game/BP/BP_Boomerang.BP_Boomerang_C"))
  (if (== OtherActor _returnvalue)
    (Default|SwitchActivated (Variables|Default|GetDoorToOpen))
    (Default|SwitchActivated (Variables|Default|GetBridgeToSpawn))
    (Components|DestroyComponent (Variables|Default|GetBox))))

(fn ConstructionScript
  (|CallParentFunction))