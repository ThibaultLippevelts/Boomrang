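; BP_GI, apparently the game instance, holds the Speed and Delay values and persists them through BP_SaveGame in a single save slot.
; Load copies both values from an existing save, or only creates an empty save object when none exists, leaving the current values untouched.
; Save stores the passed values, prints Speed, and writes a freshly created save object over the slot.
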(event Custom|Save
  (params (Speed :type Float%20%28double-precision%29) (Delay :type Float%20%28double-precision%29))
  (Variables|Default|SetDelay Delay)
  (bind _output_get (Variables|Default|SetSpeed Speed))
  (Development|PrintString (Utilities|String|ToString(Float) _output_get) true true "(R=0.286458,G=0.000000,B=0.251552,A=1.000000)")
  (bind _returnvalue (SaveGame|CreateSaveGameObject "/Game/BP/BP_SaveGame.BP_SaveGame_C"))
  (bind _output_get_2 (Variables|Default|SetSave%20game _returnvalue))
  (Variables|/Game/BP/BP_SaveGame.BP_SaveGame_C|SetSpeed _output_get_2 (Variables|Default|GetSpeed))
  (Variables|/Game/BP/BP_SaveGame.BP_SaveGame_C|SetDelay _output_get_2 (Variables|Default|GetDelay))
  (SaveGame|SaveGametoSlot _output_get_2 "Save"))

(event Custom|Load
  (bind _returnvalue (SaveGame|DoesSaveGameExist "Save"))
  (if _returnvalue
    (bind _returnvalue_2 (SaveGame|LoadGamefromSlot "Save"))
    (bind _asbp_save_game (Utilities|Casting|CastToBP_SaveGame _returnvalue_2))
    (bind _output_get (Variables|Default|SetSave%20game _asbp_save_game))
    (Variables|Default|SetSpeed (Variables|/Game/BP/BP_SaveGame.BP_SaveGame_C|GetSpeed _output_get))
    (Variables|Default|SetDelay (Variables|/Game/BP/BP_SaveGame.BP_SaveGame_C|GetDelay _output_get))
    (else
      (bind _returnvalue_3 (SaveGame|CreateSaveGameObject "/Game/BP/BP_SaveGame.BP_SaveGame_C"))
      (Variables|Default|SetSave%20game _returnvalue_3))))